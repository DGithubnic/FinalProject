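; Player State for the Murderer game that tracks skill cooldowns and stun state.
; From BeginPlay, three looping one-second timers count down two skills and an ultimate, setting each availability flag at zero.
; The flags' OnRep functions fire event dispatchers, then immediately clear the flag and restart that cooldown, so each cycle repeats automatically.
; The stun OnRep fires its own dispatcher, and MD_DTPush loads damage and hardcoded cooldown values.
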(event Custom|MD_CooltimeStart_E
  (Utilities|Time|SetTimerbyFunctionName 0 "MD_Cooltime_1_F" 1.0 true)
  (Utilities|Time|SetTimerbyFunctionName 0 "MD_Cooltime_2_F" 1.0 true)
  (Utilities|Time|SetTimerbyFunctionName 0 "MD_Ultimate_F" 1.0 true))

(event EventBeginPlay
  (CallFunction|MDCooltimeStartE))

(fn ConstructionScript)

(fn OnRepIsStun
  (if (Variables|Default|GetIsStun)
    (Default|CallPlayerStun false)
    (Development|PrintString "IsStun")))

(fn MDDTPush
  (params (MD_Damage :type Float%20%28single-precision%29) (MD_Cooltime_1 :type Float%20%28single-precision%29) (MD_Cooltime_2 :type Float%20%28single-precision%29) (MD_Ultimate :type Float%20%28single-precision%29))
  ;[1 1 1] 코멘트
  (Variables|Default|SetMD_Damage MD_Damage)
  (Variables|Default|SetMD_Cooltime_1 1e+01)
  (Variables|Default|SetMD_Cooltime_2 15.0)
  (Variables|Default|SetMD_Ultimate 2e+01))

(fn MDCooltime1F
  (bind _output_get (Variables|Default|SetMD_Cooltime_1 (Math|Float|Clamp(Float) (- (Variables|Default|GetMD_Cooltime_1) 1.0) 0.0 1e+01)))
  (if (<= _output_get 0.0)
    (Variables|Default|SetMD_CanSkill_1 true)))

(fn MDCooltime2F
  (bind _output_get (Variables|Default|SetMD_Cooltime_2 (Math|Float|Clamp(Float) (- (Variables|Default|GetMD_Cooltime_2) 1.0) 0.0 15.0)))
  (if (<= _output_get 0.0)
    (Variables|Default|SetMD_CanSkill_2 true)))

(fn MDUltimateF
  (bind _output_get (Variables|Default|SetMD_Ultimate (Math|Float|Clamp(Float) (- (Variables|Default|GetMD_Ultimate) 1.0) 0.0 2e+01)))
  (if (<= _output_get 0.0)
    (Variables|Default|SetMD_CanUltimate true)))

(fn OnRepMDCanSkill1
  (if (Variables|Default|GetMD_CanSkill_1)
    (Default|CallMDCanSkill1DP (Variables|Default|GetMD_CanSkill_1))
    (Variables|Default|SetMD_CanSkill_1 false)
    (Variables|Default|SetMD_Cooltime_1 1e+01)))

(fn OnRepMDCanSkill2
  (if (Variables|Default|GetMD_CanSkill_2)
    (Default|CallMDCanSkill2DP (Variables|Default|GetMD_CanSkill_2))
    (Variables|Default|SetMD_CanSkill_2 false)
    (Variables|Default|SetMD_Cooltime_2 15.0)))

(fn OnRepMDCanUltimate
  (if (Variables|Default|GetMD_CanUltimate)
    (Default|CallMDCanUltimateDP (Variables|Default|GetMD_CanUltimate))
    (Variables|Default|SetMD_CanUltimate false)
    (Variables|Default|SetMD_Ultimate 2e+01)))